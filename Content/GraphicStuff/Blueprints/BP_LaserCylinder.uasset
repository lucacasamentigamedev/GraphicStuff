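; BP_LaserCylinder is a visual laser beam actor built on a cylinder mesh with configurable look.
; The construction script creates a dynamic material instance on BodyCylinder and pushes the exposed color, band scroll speed, band shape and emissive intensity settings into it.
; Edits therefore update in the editor, and there is no runtime logic.
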(event `self.ReceiveBeginPlay`)

(fn `UserConstructionScript`
  (locals (BodyMaterial :type "MaterialInstanceDynamic Object Reference"))
  (`|ExecutionSequence`
    (:`then_0`
      (bind _returnvalue (`PrimitiveComponent.CreateDynamicMaterialInstance` (`self.BodyCylinder`) 0 null "None"))
      (set `local.BodyMaterial` _returnvalue))
    (:`then_1`
      (`MaterialInstanceDynamic.SetVectorParameterValue` (`local.BodyMaterial`) "Color" (`self.LaserColor`)))
    (:`then_2`
      (`MaterialInstanceDynamic.SetScalarParameterValue` (`local.BodyMaterial`) "SpeedY" (`self.SpeedY`)))
    (:`then_3`
      (`MaterialInstanceDynamic.SetScalarParameterValue` (`local.BodyMaterial`) "BandWidth" (`self.BandWidth`)))
    (:`then_4`
      (`MaterialInstanceDynamic.SetScalarParameterValue` (`local.BodyMaterial`) "BandsNumber" (`self.BandsNumber`)))
    (:`then_5`
      (`MaterialInstanceDynamic.SetScalarParameterValue` (`local.BodyMaterial`) "EmissiveIntensity" (`self.EmissiveIntensisty`)))))