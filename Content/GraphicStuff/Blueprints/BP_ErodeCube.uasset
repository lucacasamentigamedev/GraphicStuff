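; BP_ErodeCube is a cube actor that erodes away and destroys itself after being hit, also destroying the actor that hit it.
; The construction script creates a dynamic material instance on the cube mesh.
; On the first hit, a timeline drives that material's Erode scalar, with its play rate set from a random erosion time picked at BeginPlay.
; A flag ignores further hits while eroding.
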(event `self.SM_Cube.OnComponentHit`
  (params (HitComponent :type "PrimitiveComponent Object Reference") (OtherActor :type "Actor Object Reference") (OtherComp :type "PrimitiveComponent Object Reference") (NormalImpulse :type "Vector Structure") (Hit :type "HitResult Structure (by ref)"))
  ; Erode when hit
  (if (not (`self.IsEroding?`))
    (`self.K2_DestroyActor` OtherActor)
    (set `self.IsEroding?` true)
    (`TimelineComponent.SetPlayRate` (`self.TL_Erode`) (/ 1.0 (`self.ErodingTime`)))
    (bind (_direction _alpha) (`Timeline|TL_Erode` :!via `PlayFromStart`)
      (:`Update`
        (`MaterialInstanceDynamic.SetScalarParameterValue` (`self.ErodeMaterial`) "Erode" _alpha))
      (:`Finished`
        (set `self.IsEroding?` false)
        (`self.K2_DestroyActor`)))))

(event `self.ReceiveBeginPlay`
  (set `self.ErodingTime` (`KismetMathLibrary.RandomFloatInRange` 1.0 5.0)))

(fn `UserConstructionScript`
  (bind _returnvalue (`PrimitiveComponent.CreateDynamicMaterialInstance` (`self.SM_Cube`) 0 null "None"))
  (set `self.ErodeMaterial` _returnvalue))